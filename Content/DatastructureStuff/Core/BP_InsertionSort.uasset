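; BP_InsertionSort is a sorting Blueprint whose Sort function is meant to order an array ascending and return it.
; Despite its name, it uses bubble-sort-style passes, comparing each element with its predecessor and repeating until a pass needs no swap.
; The Swap call receives the predecessor's value as its second index instead of that element's position, so it does not reliably exchange neighbors.
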(fn Sort
  (params (InArray :type Array%20of%20Integers))
  (while (not (LocalVariables|GetSorted))
    (LocalVariables|SetSorted true)
    (for (_array_element _array_index) InArray
      (if (not (== _array_index 0))
        (if (< _array_element (Utilities|Array|Get(acopy) InArray (- _array_index 1)))
          (Utilities|Array|Swap InArray _array_index (Utilities|Array|Get(acopy) InArray (- _array_index 1)))
          (LocalVariables|SetSorted false)))))
  (return InArray))